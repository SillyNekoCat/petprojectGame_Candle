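; Player controller that opens the game's passive tree, pause and death menus.
; The passive tree and pause inputs create their widget as CurrentWidget, or call OnBack on the current WBP_BaseBackFunc widget if a menu is already open.
; UnPossess shows the death menu.
; Each menu pauses the game and switches to game-and-UI input with a visible cursor, while BeginPlay sets game-only input.
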(event `EnhancedInput|/Game/Input/Actions/IA_PassiveTree`
  (params (ActionValue :type Boolean) (ElapsedSeconds :type "Float (double-precision)") (TriggeredSeconds :type "Float (double-precision)") (InputAction :type "InputAction Object Reference" :default "/Game/Input/Actions/IA_PassiveTree.IA_PassiveTree"))
  ;[1 1 1] UI Passive Tree
  (:`Started`
    ;;[1 1 1] Выбираем что сделать в зависимости от того открыт сейчас какой-то виджет или нет
    (if (`self.Is_Any_Menu_Opened`)
      (bind _aswbp_base_back_func (cast `/Game/Blueprints/UI/WBP_BaseBackFunc` (`self.Current_Widget`)))
      (`/Game/Blueprints/UI/WBP_BaseBackFunc.On_Back` _aswbp_base_back_func)
      (else
        (bind _returnvalue (`|CreateWidget` "/Game/Blueprints/UI/WBP_Passive_Tree.WBP_Passive_Tree_C" self))
        (bind _output_get (set `self.Current_Widget` _returnvalue))
        (`UserWidget.AddToViewport` _output_get 0)
        (`WidgetBlueprintLibrary.SetInputMode_GameAndUIEx` self (`self.Current_Widget`))
        (set `self.bShowMouseCursor` true)
        (`GameplayStatics.SetGamePaused` true)))))

(event `EnhancedInput|/Game/Input/Actions/IA_PauseGame`
  (params (ActionValue :type Boolean) (ElapsedSeconds :type "Float (double-precision)") (TriggeredSeconds :type "Float (double-precision)") (InputAction :type "InputAction Object Reference" :default "/Game/Input/Actions/IA_PauseGame.IA_PauseGame"))
  ;[1 1 1] UI Open pause menu, back
  (:`Started`
    (if (`self.Is_Any_Menu_Opened`)
      (bind _aswbp_base_back_func (cast `/Game/Blueprints/UI/WBP_BaseBackFunc` (`self.Current_Widget`)))
      (`/Game/Blueprints/UI/WBP_BaseBackFunc.On_Back` _aswbp_base_back_func)
      (else
        (bind _returnvalue (`|CreateWidget` "/Game/Blueprints/UI/UI_Pause_Menu/WBP_Pause_Menu.WBP_Pause_Menu_C" self))
        (bind _output_get (set `self.Current_Widget` _returnvalue))
        (`UserWidget.AddToViewport` _output_get 0)
        (`WidgetBlueprintLibrary.SetInputMode_GameAndUIEx` self (`self.Current_Widget`))
        (set `self.bShowMouseCursor` true)
        (`GameplayStatics.SetGamePaused` true)))))

(event `self.ReceiveDestroyed`
  ;[1 1 1] Death Menu
)

(event `self.ReceiveUnPossess`
  (params (UnpossessedPawn :type "Pawn Object Reference"))
  ;[1 1 1] Death Menu
  (bind _returnvalue (`|CreateWidget` "/Game/Blueprints/UI/WBP_Death_Menu.WBP_Death_Menu_C" self))
  (`UserWidget.AddToViewport` _returnvalue 0)
  (`WidgetBlueprintLibrary.SetInputMode_GameAndUIEx` self _returnvalue)
  (set `self.bShowMouseCursor` true)
  (`GameplayStatics.SetGamePaused` true))

(event `self.ReceivePossess`
  (params (PossessedPawn :type "Pawn Object Reference")))

(event `self.ReceiveBeginPlay`
  (`WidgetBlueprintLibrary.SetInputMode_GameOnly` self))

(fn `UserConstructionScript`)
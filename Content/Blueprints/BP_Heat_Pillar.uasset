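; BP_Heat_Pillar is a pillar actor with a HeatComponent and an optional on-screen readout of its heat state.
; When HeatDebug is set, the construction script adds two text render components, and Tick writes accumulated heat and the heat status parameter to them.
; BeginPlay, overlap and max-heat events are empty stubs, so this graph only drives the debug display.
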(event `self.ReceiveBeginPlay`)

(event `self.ReceiveActorBeginOverlap`
  (params (OtherActor :type "Actor Object Reference")))

(event `OnMax_Heat_Delegate_Event`)

(event `self.ReceiveTick`
  (params (DeltaSeconds :type "Float (single-precision)"))
  (if (`self.Heat_Debug`)
    (`TextRenderComponent.K2_SetText` (`self.Text_Comp_0`) (`KismetTextLibrary.Conv_DoubleToText` (`Heat_Component.Accumulated_Heat` (`self.Heat_Component`)) "HalfToEven"))
    (`TextRenderComponent.K2_SetText` (`self.Text_Comp_2_0`) (`KismetTextLibrary.Conv_DoubleToText` (`Heat_Component.Heat_Status_Param` (`self.Heat_Component`)) "HalfToEven"))))

(fn `UserConstructionScript`
  (if (`self.Heat_Debug`)
    (bind _returnvalue (`AddComponent|NODE_AddTextRenderComponent-0` :`RelativeTransform` (`KismetMathLibrary.MakeTransform` (60.0 35.0 -5.0))))
    (set `self.Text_Comp_0` _returnvalue)
    (bind _returnvalue_2 (`AddComponent|NODE_AddTextRenderComponent-1` :`RelativeTransform` (`KismetMathLibrary.MakeTransform` (60.0 35.0 25.0))))
    (set `self.Text_Comp_2_0` _returnvalue_2)))
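; Logic door that slides Cube0 open by an end offset when its button condition and optional heat condition are met, and closes it otherwise.
; Button changes update a gate that requires all buttons active; if a heat type is set, all heat must also exceed the minimum.
; Heat check events re-evaluate using the cached button gate.
; A timeline plays or reverses to lerp the cube from its BeginPlay relative location.
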(event `self.Button_ActivationChange`
  (params (new_value :type Boolean))
  (switch `/Game/Blueprints/Enums/Enum_ButtonActivationType` (`self.Button_Activation_Type`)
    (:`NewEnumerator6`
      (bind _result (`self.Is_All_Buttons_Active`))
      (set `self.Buttons_Gate` _result)
      (if (`|EnumEquality` (`self.Heat_Activation_Type`) "NewEnumerator6")
        (if (`self.Buttons_Gate`)
          (bind (_direction _door_relative_location) (`Timeline|Timeline_0` :!label _label)
            (:`Update`
              (`SceneComponent.K2_SetRelativeLocation` (`self.Cube_0`) (`KismetMathLibrary.VLerp` (`self.Cube Start Relative Location`) (+ (`self.Cube Start Relative Location`) (`self.End_Offset`)) _door_relative_location) false false)))
          (else
            (goto _label :!via `Reverse`)))
        (else
          (if (`self.Buttons_Gate`) :!label _label_2
            (switch `/Game/Blueprints/Enums/Enum_HeatAtcivationType` (`self.Heat_Activation_Type`)
              (:`NewEnumerator2`
                (bind _is_all_greater (`self.Is_AllGreaterThan_MinHeat`))
                (if _is_all_greater
                  (goto _label)
                  (else
                    (goto _label :!via `Reverse`)))))
            (else
              (goto _label :!via `Reverse`))))))))

(event `self.Event_All_CheckHeat`
  (params (heat_status :type "Float (double-precision)"))
  (goto _label_2))

(event `self.ReceiveBeginPlay`
  (`parent.ReceiveBeginPlay`)
  (set `self.Cube Start Relative Location` (`SceneComponent.RelativeLocation` (`self.Cube_0`))))

(fn `UserConstructionScript`
  (`parent.UserConstructionScript`))
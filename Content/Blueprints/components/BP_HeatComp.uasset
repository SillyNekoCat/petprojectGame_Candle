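; Heat component that listens for damage taken by its owning actor through the Gameplay Ability System.
; On BeginPlay it gets the owner's Base_AttributeSet from its ability system component and binds to the set's damage-take delegate.
; Each damage event passes instigator, causer, tag, amount and old and new values straight to HeatDamageTake, whose logic is not in this graph.
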(event `self.ReceiveBeginPlay`
  (set `self.Owner` (`self.GetOwner`))
  (bind _returnvalue (`AbilitySystemComponent.GetAttributeSet` (`AbilitySystemBlueprintLibrary.GetAbilitySystemComponent` (`self.Owner`)) "/Script/Living_Candle.Base_AttributeSet"))
  (bind _asbase_attribute_set (cast `Base_AttributeSet` _returnvalue))
  (set `self.Owner_Base_AttributeSet` _asbase_attribute_set)
  (add `Base_AttributeSet.On_Damage_Take` (`self.Owner_Base_AttributeSet`) (delegate `On_Damage_Take_Event`)))

(event `On_Damage_Take_Event`
  (params (EffectInstigator :type "Actor Object Reference") (EffectCauser :type "Actor Object Reference") (DamageTag :type "GameplayTag Structure") (Damage :type "Float (single-precision)") (OldValue :type "Float (single-precision)") (NewValue :type "Float (single-precision)"))
  (`self.HeatDamage_Take` EffectInstigator EffectCauser DamageTag Damage OldValue NewValue))
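; Floating health bar widget component that shows its owner's health, last hit, total damage and DPS.
; It binds to the damage event on the owner's Base_AttributeSet and pushes values into WBP_Floating_HealthBar, resetting damage totals after a few seconds without hits.
; A looping timer shows the bar only while the owner is on the damaging player's screen, stopping after a spell out of sight; a debug flag keeps it visible.
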(event `self.ReceiveBeginPlay`
  (`|ExecutionSequence`
    (:`then_0`
      ;[1 1 1] Setup Data
      (set `self.Owner` (`self.GetOwner`))
      (bind _aswbp_floating_health_bar (cast `/Game/Blueprints/UI/WBP_Floating_HealthBar` (`self.GetUserWidgetObject`))
        (:`then`
          (set `self.HealthBar_Widget` _aswbp_floating_health_bar)
          (bind _returnvalue (`AbilitySystemComponent.GetAttributeSet` (`AbilitySystemBlueprintLibrary.GetAbilitySystemComponent` (`self.Owner`)) "/Script/Living_Candle.Base_AttributeSet"))
          (bind _asbase_attribute_set (cast `Base_AttributeSet` _returnvalue)
            (:`then`
              (set `self.Owner_Base_AttributeSet` _asbase_attribute_set)
              (add `Base_AttributeSet.On_RecieveDamage` (`self.Owner_Base_AttributeSet`) (delegate `On_RecieveDamage_Event`)))
            (:`CastFailed`
              (`KismetSystemLibrary.PrintString` "Base_Attr cast fail"))))
        (:`CastFailed`
          (`KismetSystemLibrary.PrintString` "WBP FloatingHealth cast fail"))))
    (:`then_1`
      (`self.UpdateWidget_HealthBar`)
      (if (`self.Is_Visible_AllTime_DEBUG`)
        (`self.Set_HealthBarVisibility` true)
        (else
          (`self.Set_HealthBarVisibility` false))))))

(event `On_RecieveDamage_Event`
  (params (EffectInstigator :type "Actor Object Reference") (EffectCauser :type "Actor Object Reference") (Damage_Info :type "Damage_Info Structure"))
  (bind (_phys_damage _fire_damage _pure_damage) (break `Damage_Info` Damage_Info))
  (bind _returnvalue (+ _phys_damage _fire_damage _pure_damage))
  (`|ExecutionSequence`
    (:`then_0`
      (`self.UpdateWidget_LastHit` _returnvalue)
      (`self.Add_TotalDamage` _returnvalue)
      (`self.DPS` (`self.Total_Damage`))
      (`self.UpdateWidget_HealthBar`)
      (if (not (`self.Is_Visible_AllTime_DEBUG`))
        (bind _output_get (set `self.Last_Damage_Actor` EffectCauser))
        (`self.Check_Sight` _output_get)
        (`self.SetTimer_SightCheckLoop`)))))

(fn `Add_TotalDamage`
  (params (new_damage :type "Float (double-precision)"))
  (bind _output_get (set `self.Total_Damage` (+ new_damage (`self.Total_Damage`))))
  (`self.UpdateWidget_TotalDamage` _output_get))

(fn `Check_Sight`
  (params (actor :type "Actor Object Reference"))
  (returns (is_visible :type Boolean))
  (bind _instigator (`Actor.Instigator` actor))
  (`/Engine/EditorBlueprintResources/StandardMacros.IsValid` _instigator
    (:`Is Valid`
      (if (`Pawn.IsPlayerControlled` _instigator)
        (bind _returnvalue (`R_BP_FunctionLibrary.Is_On_Screen` (`self.Owner`) (`PlayerState.GetPlayerController` (`Pawn.PlayerState` _instigator))))
        (if _returnvalue
          (`self.Set_HealthBarVisibility` true)
          (return true)
          (else
            (`self.Set_HealthBarVisibility` false)
            (return false)))))))

(fn `DPS`
  (params (new_damage :type "Float (double-precision) (by ref)"))
  (`|ExecutionSequence`
    (:`then_0`
      (if (`KismetSystemLibrary.K2_IsTimerActiveHandle` (`self.DPS_TimerHandle`))
        (`self.UpdateWidget_DPS` (/ (`self.Total_Damage`) (+ (`KismetSystemLibrary.K2_GetTimerElapsedTimeHandle` (`self.DPS_TimerHandle`)) (`self.Total_ElapsedTime`))))
        (else
          (`self.UpdateWidget_DPS` new_damage))))
    (:`then_1`
      (`self.SetTimer_DPS`))))

(fn `DPS_Timer`
  (set `self.Total_Damage` 0.0)
  (set `self.Total_ElapsedTime` 0.0)
  (`self.UpdateWidget_DPS` 0.0)
  (`self.UpdateWidget_TotalDamage` 0.0))

(fn `Set_HealthBarVisibility`
  (params (is_visible :type Boolean))
  (bind _healthbar_widget (`self.HealthBar_Widget`))
  (bind _textblock_dps (`/Game/Blueprints/UI/WBP_Floating_HealthBar.TextBlock_DPS` (`self.HealthBar_Widget`)))
  (bind _textblock_totaldamage (`/Game/Blueprints/UI/WBP_Floating_HealthBar.TextBlock_TotalDamage` (`self.HealthBar_Widget`)))
  (`|ExecutionSequence`
    (:`then_0`
      (if (`self.isShow_DPS_TotalDamage`)
        (`Widget.SetVisibility` _textblock_totaldamage "Visible")
        (`Widget.SetVisibility` _textblock_dps "Visible")
        (else
          (`Widget.SetVisibility` _textblock_totaldamage "Hidden")
          (`Widget.SetVisibility` _textblock_dps "Hidden"))))
    (:`then_1`
      (if is_visible
        (`Widget.SetVisibility` _healthbar_widget "Visible")
        (else
          (`Widget.SetVisibility` _healthbar_widget "Hidden"))))))

(fn `SetTimer_DPS`
  (set `self.Total_ElapsedTime` (+ (`self.Total_ElapsedTime`) (`KismetSystemLibrary.K2_GetTimerElapsedTimeHandle` (`self.DPS_TimerHandle`))))
  (bind _returnvalue (`KismetSystemLibrary.K2_SetTimer` null "DPS_Timer" 4.0))
  (set `self.DPS_TimerHandle` _returnvalue))

(fn `SetTimer_SightCheckLoop`
  (`KismetSystemLibrary.K2_ClearAndInvalidateTimerHandle` (`self.SightCheckLoop_Handle`))
  (bind _returnvalue (`KismetSystemLibrary.K2_SetTimer` null "Sight_Check_Loop" (`self.Timer_Sight_Check_Interval`) true))
  (set `self.SightCheckLoop_Handle` _returnvalue))

(fn `Sight_Check_Duration`
  (`KismetSystemLibrary.K2_ClearAndInvalidateTimerHandle` (`self.SightCheckLoop_Handle`))
  (`KismetSystemLibrary.K2_ClearAndInvalidateTimerHandle` (`self.SightCheckDuration_Handle`)))

(fn `Sight_Check_Loop`
  (bind _is_visible (`self.Check_Sight` (`self.Last_Damage_Actor`)))
  (if _is_visible
    ;[1 1 1] Reset checking loop duration if owner is in sight
    (`KismetSystemLibrary.K2_ClearAndInvalidateTimerHandle` (`self.SightCheckDuration_Handle`))
    (bind _returnvalue (`KismetSystemLibrary.K2_SetTimer` null "Sight_Check_Duration" (`self.Timer_Sight_Check_Duration`)))
    (set `self.SightCheckDuration_Handle` _returnvalue)))

(fn `UpdateWidget_DPS`
  (params (input :type "Float (double-precision)"))
  (set `/Game/Blueprints/UI/WBP_Floating_HealthBar.DPS` input (`self.HealthBar_Widget`)))

(fn `UpdateWidget_HealthBar`
  (bind _healthbar_widget (`self.HealthBar_Widget`))
  (bind _owner_base_attributeset (`self.Owner_Base_AttributeSet`))
  (set `/Game/Blueprints/UI/WBP_Floating_HealthBar.w_current_hp` (`.CurrentValue` (break `GameplayAttributeData` (`Base_AttributeSet.Health` _owner_base_attributeset))) _healthbar_widget)
  (set `/Game/Blueprints/UI/WBP_Floating_HealthBar.w_max_hp` (`.CurrentValue` (break `GameplayAttributeData` (`Base_AttributeSet.Health_Max` _owner_base_attributeset))) _healthbar_widget))

(fn `UpdateWidget_LastHit`
  (params (input :type "Float (double-precision)"))
  (set `/Game/Blueprints/UI/WBP_Floating_HealthBar.Last_Hit` input (`self.HealthBar_Widget`)))

(fn `UpdateWidget_TotalDamage`
  (params (input :type "Float (double-precision)"))
  (set `/Game/Blueprints/UI/WBP_Floating_HealthBar.Total_Damage` input (`self.HealthBar_Widget`)))
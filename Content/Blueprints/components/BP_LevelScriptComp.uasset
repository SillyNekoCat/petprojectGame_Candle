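; Level-script component that aggregates heat targets and buttons to drive puzzle-style mechanisms.
; On BeginPlay it subscribes to every target and relays heat and button changes through its own dispatchers, opening the button gate when no buttons exist or certain activation types apply.
; Helpers evaluate minimum heat, average heat and all-buttons-active, and compute a clamped, reversible speed.
; Bind hooks consumers to both dispatchers and immediately broadcasts zero heat and inactive state.
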(event `self.ReceiveBeginPlay`
  (`self.Bind_ForAllTargets`)
  (if (or (`KismetArrayLibrary.Array_IsEmpty` (`self.Button_Targets`)) (`|EnumEquality` (`self.Button_Activation_Type`) "NewEnumerator2") (`|EnumEquality` (`self.Button_Activation_Type`) "NewEnumerator8"))
    (set `self.Buttons_Gate` true)
    (`self.Event_All_CheckHeat` 0.0)))

(event `Bind_ForAllTargets`
  (`|ExecutionSequence`
    (:`then_0`
      (for _array_element (`self.Heat_Targets`)
        (`/Engine/EditorBlueprintResources/StandardMacros.IsValid` _array_element
          (:`Is Valid`
            (add `Heat_Actor.OnCheckHeat_Delegate` _array_element (delegate `Event_All_CheckHeat`))))))
    (:`then_1`
      (for _array_element_2 (`self.Button_Targets`)
        (`/Engine/EditorBlueprintResources/StandardMacros.IsValid` _array_element_2
          (:`Is Valid`
            (add `/Game/Blueprints/BP_Button.Button_ActivationChange_Delegate` _array_element_2 (delegate `Button_ActivationChange`))))))))

(event `Event_All_CheckHeat`
  (params (heat_status :type "Float (double-precision)"))
  (`self.On_All_CheckHeat` heat_status))

(event `Button_ActivationChange`
  (params (is_active :type Boolean))
  (`self.On_Button_Activation_Change` is_active))

(fn `Bind`
  (params (On_All_CheckHeat :type "Delegate (by ref)") (On_Button_Activation_Change :type "Delegate (by ref)"))
  (add `self.On_All_CheckHeat` On_All_CheckHeat)
  (add `self.On_Button_Activation_Change` On_Button_Activation_Change)
  (`self.On_All_CheckHeat` 0.0)
  (`self.On_Button_Activation_Change` false))

(fn `Calc_AverageHeat`
  (returns (avarage_heat_value :type "Float (double-precision)"))
  (locals (sum :type "Float (double-precision)"))
  (bind _heat_targets (`self.Heat_Targets`))
  (for _array_element _heat_targets
    (set `local.sum` (+ (`local.sum`) (`Heat_Component.Heat_Status_Param` (`Actor.GetComponentByClass` _array_element "/Game/Blueprints/components/BP_HeatComp.BP_HeatComp_C")))))
  (return (/ (`local.sum`) (`KismetArrayLibrary.Array_Length` _heat_targets))))

(fn `Is_All_Buttons_Active`
  (returns (result :type Boolean))
  (for _array_element (`self.Button_Targets`)
    (if (not (`/Game/Blueprints/BP_Button.Is_Active` _array_element))
      (return false)))
  (return true))

(fn `Is_AllGreaterThan_MinHeat`
  (returns (is_all_greater :type Boolean))
  (locals (all_heat_params :type "Array of Float (double-precision)"))
  (for _array_element (`self.Heat_Targets`)
    (`KismetArrayLibrary.Array_Add` (`local.all_heat_params`) (`Heat_Component.Heat_Status_Param` (`Actor.GetComponentByClass` _array_element "/Game/Blueprints/components/BP_HeatComp.BP_HeatComp_C"))))
  (for _array_element_2 (`local.all_heat_params`)
    (if (< _array_element_2 (`self.Min_Heat`))
      (return false)))
  (return true))

(fn `Set_Reverse`
  (params (new_value :type Boolean))
  (set `self.Reverse` new_value)
  (`self.Set_Speed` (`self.Current_Speed`)))

(fn `Set_Speed`
  (params (new_speed :type "Float (double-precision)"))
  (locals (input_speed :type "Float (double-precision)"))
  (set `local.input_speed` new_speed)
  (if (`self.Reverse`)
    (set `self.Current_Speed` (`KismetMathLibrary.FMax` (* (`self.FullPower_Speed`) -1.0) (* (+ (`self.Min_Speed`) (`local.input_speed`)) -1.0)))
    (else
      (set `self.Current_Speed` (`KismetMathLibrary.FMin` (`self.FullPower_Speed`) (+ (`self.Min_Speed`) (`KismetMathLibrary.Abs` (`local.input_speed`))))))))
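; BP_LogicDoorTwo is a door that slides open in response to heat reported by two linked targets.
; It binds to each target's heat delegate; a status of 1.0 or above plays a shared Timeline, otherwise it reverses.
; The Timeline lerps the Cube's relative location from its start to an end offset.
; Each handler tests only its own status, twice, so the latest report alone sets the door's direction.
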(event `self.ReceiveBeginPlay`
  (set `self.Cube Start Relative Location` (`SceneComponent.RelativeLocation` (`self.Cube`)))
  (add `Heat_Actor.OnCheckHeat_Delegate` (`self.Target1`) (delegate `OnCheckHeat_Delegate_Event1`))
  (add `Heat_Actor.OnCheckHeat_Delegate` (`self.Target2`) (delegate `OnCheckHeat_Delegate_Event2`)))

(event `OnCheckHeat_Delegate_Event1`
  (params (heat_status :type "Float (double-precision)"))
  (if (and (>= heat_status 1.0) (>= (stale `OnCheckHeat_Delegate_Event2` heat_status) 1.0))
    (bind (_direction _door_relative_location) (`Timeline|Timeline` :!label _label)
      (:`Update`
        (`SceneComponent.K2_SetRelativeLocation` (`self.Cube`) (`KismetMathLibrary.VLerp` (`self.Cube Start Relative Location`) (+ (`self.Cube Start Relative Location`) (`self.End_Offset`)) _door_relative_location) false false)))
    (else
      (goto _label :!via `Reverse`))))

(event `OnCheckHeat_Delegate_Event2`
  (params (heat_status :type "Float (double-precision)"))
  (if (and (>= (stale `OnCheckHeat_Delegate_Event1` heat_status) 1.0) (>= heat_status 1.0))
    (goto _label)
    (else
      (goto _label :!via `Reverse`))))

(fn `UserConstructionScript`)
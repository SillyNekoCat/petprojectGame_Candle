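; Base AI character Blueprint that uses the Gameplay Ability System for melee combat and health.
; On BeginPlay it binds attribute-set health events, grants a serial melee ability and equips a mace through its attack component.
; Zero health destroys the actor, while damage and health-change handlers are empty.
; It also provides a looping random-wander event, a walk-speed setter and an Attack function that activates melee abilities by tag.
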(event `NPC_RandomMove`
  (`|AIMoveTo` self (`NavigationSystemV1.K2_GetRandomReachablePointInRadius` (`self.K2_GetActorLocation`) 3000.0 null null) null 70.0
    (:`OnSuccess`
      (`KismetSystemLibrary.Delay` (`KismetMathLibrary.RandomFloatInRange` 0.1 6.0))
      (`self.NPC_RandomMove`))
    (:`OnFail`
      (`KismetSystemLibrary.Delay` 0.1)
      (`self.NPC_RandomMove`))))

(event `self.ReceiveTick`
  (params (DeltaSeconds :type "Float (single-precision)")))

(event `self.ReceiveBeginPlay`
  (`self.Bind_Health_Events`)
  (`AbilitySystemComponent.K2_GiveAbility` (`self.AbilitySystem_Comp`) "/Game/Blueprints/Ability_System/Ability/GA_Melee_SerialAttack.GA_Melee_SerialAttack_C" 0 -1)
  (`/Game/Blueprints/components/BP_AttackComp.Give_Weapon` (`self.AttackComp`) "/Game/Blueprints/BP_Macee.BP_Macee_C" false true 2.0 5.0 true))

(event `Bind_Health_Events`
  (bind _asc_baseattributeset (`self.asc_BaseAttributeSet`))
  (`|ExecutionSequence`
    (:`then_0`
      (bind _returnvalue (`AbilitySystemComponent.GetAttributeSet` (`self.AbilitySystem_Comp`) "/Script/Living_Candle.Base_AttributeSet"))
      (bind _asbase_attribute_set (cast `Base_AttributeSet` _returnvalue))
      (set `self.asc_BaseAttributeSet` _asbase_attribute_set))
    (:`then_1`
      (add `Base_AttributeSet.On_Damage_Take` _asc_baseattributeset (`|CreateDelegate` :!event `On_Damage_Take_Event_1`))
      (add `Base_AttributeSet.On_Health_Changed` _asc_baseattributeset (`|CreateDelegate` :!event `On_Health_Changed_Event`))
      (add `Base_AttributeSet.On_Health_Zero` _asc_baseattributeset (`|CreateDelegate` :!event `On_Health_Zero_Event`)))))

(event `On_Damage_Take_Event_1`
  (params (EffectInstigator :type "Actor Object Reference") (EffectCauser :type "Actor Object Reference") (DamageTag :type "GameplayTag Structure") (Magnitude :type "Float (single-precision)") (OldValue :type "Float (single-precision)") (NewValue :type "Float (single-precision)")))

(event `On_Health_Changed_Event`
  (params (EffectInstigator :type "Actor Object Reference") (EffectCauser :type "Actor Object Reference") (DamageTag :type "GameplayTag Structure") (Magnitude :type "Float (single-precision)") (OldValue :type "Float (single-precision)") (NewValue :type "Float (single-precision)")))

(event `On_Health_Zero_Event`
  (params (EffectInstigator :type "Actor Object Reference") (EffectCauser :type "Actor Object Reference") (DamageTag :type "GameplayTag Structure") (Magnitude :type "Float (single-precision)") (OldValue :type "Float (single-precision)") (NewValue :type "Float (single-precision)"))
  (`self.K2_DestroyActor`))

(fn `Attack`
  (returns (was_activated :type Boolean))
  (bind _returnvalue (`AbilitySystemComponent.TryActivateAbilitiesByTag` (`self.AbilitySystem_Comp`) (`BlueprintGameplayTagLibrary.MakeLiteralGameplayTagContainer` (struct :`GameplayTags` (struct :`(TagName` "Ability.Melee_Attack")))) true))
  (return _returnvalue))

(fn `Update Walk Speed`
  (params (NewWalkSpeed :type "Float (double-precision)"))
  (set `CharacterMovementComponent.MaxWalkSpeed` NewWalkSpeed (`self.CharacterMovement`)))

(fn `UserConstructionScript`)
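; NPC character Blueprint built on the Gameplay Ability System, with walk speed read from a gameplay attribute.
; BeginPlay grants light and heavy melee attack abilities and binds damage, health-changed and health-zero events from the Base_AttributeSet.
; Those health handlers are empty stubs, and a random wander loop using AIMoveTo is disconnected, so it never runs.
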(event `NPC_RandomMove`)

(event `self.ReceiveTick`
  (params (DeltaSeconds :type "Float (single-precision)")))

(event `self.ReceiveBeginPlay`
  (set `CharacterMovementComponent.MaxWalkSpeed` (`.ReturnValue` (`AbilitySystemComponent.GetGameplayAttributeValue` (`self.AbilitySystem_Comp`) (struct :`AttributeName` "Move_Speed" :`Attribute` "/Script/Living_Candle.Movement_AttributeSet:Move_Speed" :`AttributeOwner` "/Script/CoreUObject.Class'/Script/Living_Candle.Movement_AttributeSet'"))) (`self.CharacterMovement`))
  (`self.Bind_Health_Events`)
  (`AbilitySystemComponent.K2_GiveAbility` (`self.AbilitySystem_Comp`) "/Game/Blueprints/Ability_System/Ability/GA_Melee_LightAttack.GA_Melee_LightAttack_C" 0 -1)
  (`AbilitySystemComponent.K2_GiveAbility` (`self.AbilitySystem_Comp`) "/Game/Blueprints/Ability_System/Ability/GA_Melee_HeavyAttack.GA_Melee_HeavyAttack_C" 0 -1))

(event `Bind_Health_Events`
  (bind _asc_baseattributeset (`self.asc_BaseAttributeSet`))
  (`|ExecutionSequence`
    (:`then_0`
      (bind _returnvalue (`AbilitySystemComponent.GetAttributeSet` (`self.AbilitySystem_Comp`) "/Script/Living_Candle.Base_AttributeSet"))
      (bind _asbase_attribute_set (cast `Base_AttributeSet` _returnvalue))
      (set `self.asc_BaseAttributeSet` _asbase_attribute_set))
    (:`then_1`
      (add `Base_AttributeSet.On_RecieveDamage` _asc_baseattributeset (`|CreateDelegate` :!event `On_RecieveDamage_Event`))
      (add `Base_AttributeSet.On_Health_Changed` _asc_baseattributeset (`|CreateDelegate` :!event `On_Health_Changed_Event`))
      (add `Base_AttributeSet.On_Health_Zero` _asc_baseattributeset (`|CreateDelegate` :!event `On_Health_Zero_Event`)))))

(event `On_RecieveDamage_Event`
  (params (EffectInstigator :type "Actor Object Reference") (EffectCauser :type "Actor Object Reference") (Damage_Info :type "Damage_Info Structure")))

(event `On_Health_Changed_Event`
  (params (EffectInstigator :type "Actor Object Reference") (EffectCauser :type "Actor Object Reference") (DamageTag :type "GameplayTag Structure") (Magnitude :type "Float (single-precision)") (OldValue :type "Float (single-precision)") (NewValue :type "Float (single-precision)")))

(event `On_Health_Zero_Event`
  (params (EffectInstigator :type "Actor Object Reference") (EffectCauser :type "Actor Object Reference") (DamageTag :type "GameplayTag Structure") (Magnitude :type "Float (single-precision)") (OldValue :type "Float (single-precision)") (NewValue :type "Float (single-precision)")))

(fn `UserConstructionScript`)
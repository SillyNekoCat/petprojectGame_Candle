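; Prototype flame stream actor that detects targets along a line from its start component to an End point placed by Length.
; BeginPlay fits a capsule around the stream, and an overlap starts a looping sphere-trace timer between the endpoints, with debug drawing.
; Traces collect hit actors, skipping interact spheres, but damage is not applied because that loop is disconnected.
; The trace and a slower Sleep timer clear both timers once the capsule empties.
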(event `self.ReceiveBeginPlay`
  (bind _returnvalue (`KismetMathLibrary.VSize` (- (`self.Start_Loc0`) (`self.End_Loc0`))))
  (set `self.Start_Loc0` (`SceneComponent.K2_GetComponentLocation` (`self.Start(FlameCompPrototype)`)))
  (set `self.End_Loc0` (`SceneComponent.K2_GetComponentLocation` (`self.End`)))
  (`CapsuleComponent.SetCapsuleRadius` (`self.Capsule`) (`self.Radius0`) true)
  (`CapsuleComponent.SetCapsuleHalfHeight` (`self.Capsule`) (+ (/ _returnvalue 2.0) (`self.Radius0`)) true)
  (`SceneComponent.K2_AddLocalOffset` (`self.Capsule`) (`KismetMathLibrary.MakeVector` 0.0 0.0 (/ _returnvalue 2.0)) false false))

(event `self.ReceiveTick`
  (params (DeltaSeconds :type "Float (single-precision)")))

(event `self.Capsule.OnComponentBeginOverlap`
  (params (OverlappedComponent :type "PrimitiveComponent Object Reference") (OtherActor :type "Actor Object Reference") (OtherComp :type "PrimitiveComponent Object Reference") (OtherBodyIndex :type Integer) (bFromSweep :type Boolean) (SweepResult :type "HitResult Structure (by ref)"))
  (set `self.overlaping_actors0` (`PrimitiveComponent.GetOverlappingActors` (`self.Capsule`) null))
  (bind _returnvalue (`KismetSystemLibrary.K2_SetTimer` null "Sleep" 5.0 true))
  (set `self.Sleep_TimerHandle0` _returnvalue)
  (if (not (`KismetSystemLibrary.K2_IsTimerActiveHandle` (`self.DealingDamage_TimerHandle0`)))
    (bind _returnvalue_2 (`KismetSystemLibrary.K2_SetTimer` null "Dealing_Damage" (`self.Trace_Interval`) true))
    (set `self.DealingDamage_TimerHandle0` _returnvalue_2)))

(event `self.Capsule.OnComponentEndOverlap`
  (params (OverlappedComponent :type "PrimitiveComponent Object Reference") (OtherActor :type "Actor Object Reference") (OtherComp :type "PrimitiveComponent Object Reference") (OtherBodyIndex :type Integer)))

(fn `Dealing_Damage`
  (set `self.Start_Loc0` (`SceneComponent.K2_GetComponentLocation` (`self.Start(FlameCompPrototype)`)))
  (set `self.End_Loc0` (`SceneComponent.K2_GetComponentLocation` (`self.End`)))
  (bind _outhits (`KismetSystemLibrary.SphereTraceMultiByProfile` :`Start` (`self.Start_Loc0`) :`End` (`self.End_Loc0`) :`Radius` (`self.Radius0`) :`ProfileName` "OverlapOnlyPawn" :`DrawDebugType` "ForDuration" :`DrawTime` (`self.Trace_Interval`)))
  (for _array_element _outhits
    (bind (_bblockinghit _binitialoverlap _time _distance _location _impactpoint _normal _impactnormal _physmat _hitactor _hitcomponent) (`GameplayStatics.BreakHitResult` _array_element))
    (if (not (`.bSuccess` (cast `Interact_SphereComponent` _hitcomponent :!pure true)))
      (`KismetArrayLibrary.Array_AddUnique` (`self.Damage_Actors0`) _hitactor)))
  (set `self.overlaping_actors0` (`PrimitiveComponent.GetOverlappingActors` (`self.Capsule`) null))
  (if (== (`KismetArrayLibrary.Array_Length` (`self.overlaping_actors0`)) 0)
    (`KismetSystemLibrary.K2_ClearAndInvalidateTimerHandle` (`self.DealingDamage_TimerHandle0`))
    (`KismetSystemLibrary.K2_ClearAndInvalidateTimerHandle` (`self.Sleep_TimerHandle0`))))

(fn `GetAndValidate_OverlapingComp`
  (bind _output_get (set `self.Overlapping_Components` (`PrimitiveComponent.GetOverlappingComponents` (`self.Capsule`))))
  (for _array_element _output_get
    (cast `Interact_SphereComponent` _array_element)
    (`KismetArrayLibrary.Array_RemoveItem` (`self.Overlapping_Components`) _array_element)))

(fn `Sleep`
  (set `self.overlaping_actors0` (`PrimitiveComponent.GetOverlappingActors` (`self.Capsule`) null))
  (if (== (`KismetArrayLibrary.Array_Length` (`self.overlaping_actors0`)) 0)
    (`KismetSystemLibrary.K2_ClearAndInvalidateTimerHandle` (`self.DealingDamage_TimerHandle0`))
    (`KismetSystemLibrary.K2_ClearAndInvalidateTimerHandle` (`self.Sleep_TimerHandle0`))))

(fn `UserConstructionScript`
  (`SceneComponent.K2_SetRelativeLocation` (`self.End`) (`KismetMathLibrary.MakeVector` 0.0 0.0 (`self.Length`)) false false))
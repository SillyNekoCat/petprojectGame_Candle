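; BP_Heat_Cube1 is a cube actor with a HeatComponent and an optional on-actor debug readout of its heat state.
; When HeatDebug is set, the construction script adds two text render components, and Tick writes AccumulatedHeat and HeatStatusParam to them.
; The overlap events are empty, and leftover physics-disable and pickup name-check nodes are never executed.
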(event `self.ReceiveBeginPlay`)

(event `self.ReceiveActorBeginOverlap`
  (params (OtherActor :type "Actor Object Reference")))

(event `self.ReceiveTick`
  (params (DeltaSeconds :type "Float (single-precision)"))
  (if (`self.Heat_Debug`)
    (`TextRenderComponent.K2_SetText` (`self.Text_Comp`) (`KismetTextLibrary.Conv_DoubleToText` (`Heat_Component.Accumulated_Heat` (`self.Heat_Component`)) "HalfToEven"))
    (`TextRenderComponent.K2_SetText` (`self.Text_Comp_2`) (`KismetTextLibrary.Conv_DoubleToText` (`Heat_Component.Heat_Status_Param` (`self.Heat_Component`)) "HalfToEven"))))

(event `self.Box.OnComponentBeginOverlap`
  (params (OverlappedComponent :type "PrimitiveComponent Object Reference") (OtherActor :type "Actor Object Reference") (OtherComp :type "PrimitiveComponent Object Reference") (OtherBodyIndex :type Integer) (bFromSweep :type Boolean) (SweepResult :type "HitResult Structure (by ref)")))

(event `self.Cube.OnComponentBeginOverlap`
  (params (OverlappedComponent :type "PrimitiveComponent Object Reference") (OtherActor :type "Actor Object Reference") (OtherComp :type "PrimitiveComponent Object Reference") (OtherBodyIndex :type Integer) (bFromSweep :type Boolean) (SweepResult :type "HitResult Structure (by ref)")))

(fn `UserConstructionScript`
  (if (`self.Heat_Debug`)
    (bind _returnvalue (`AddComponent|NODE_AddTextRenderComponent-0` :`RelativeTransform` (`KismetMathLibrary.MakeTransform` (60.0 35.0 -5.0))))
    (set `self.Text_Comp` _returnvalue)
    (bind _returnvalue_2 (`AddComponent|NODE_AddTextRenderComponent-1` :`RelativeTransform` (`KismetMathLibrary.MakeTransform` (60.0 35.0 25.0))))
    (set `self.Text_Comp_2` _returnvalue_2)))
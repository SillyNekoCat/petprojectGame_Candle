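; Heat-reactive cube actor that responds to Fire damage received through the Gameplay Ability System.
; It binds to its Base_AttributeSet's damage delegate, and Fire-tagged hits run a heat melting check and set a contact-damage timer, using functions defined outside these graphs.
; With Debug on, construction adds two text renders showing the HeatComponent's accumulated heat and status value, refreshed by the heat-check delegate.
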(event `self.ReceiveBeginPlay`
  (bind _returnvalue (`AbilitySystemComponent.GetAttributeSet` (`self.AbilitySystem_Comp`) "/Script/Living_Candle.Base_AttributeSet"))
  (bind _asbase_attribute_set (cast `Base_AttributeSet` _returnvalue))
  (bind _output_get (set `self.Base_AttributeSet_BP` _asbase_attribute_set))
  (add `Base_AttributeSet.On_Damage_Take` _output_get (delegate `On_Damage_Take_Event`))
  (add `self.OnCheckHeat_Delegate` (delegate `OnCheckHeat_Delegate_Event`)))

(event `OnCheckHeat_Delegate_Event` :!signature `self.OnCheckHeat_Delegate`
  (params (heat_status :type "Float (double-precision)"))
  (`self.Debug_Heat`))

(event `On_Damage_Take_Event`
  (params (EffectInstigator :type "Actor Object Reference") (EffectCauser :type "Actor Object Reference") (DamageTag :type "GameplayTag Structure") (Magnitude :type "Float (single-precision)") (OldValue :type "Float (single-precision)") (NewValue :type "Float (single-precision)"))
  (if (== DamageTag (struct :`TagName` "DamageTypes.Fire"))
    (`self.Check_HeatMelting`)
    (`self.Set_CheckContactDamage_Timer`)))

(event `self.ReceiveActorBeginOverlap`
  (params (OtherActor :type "Actor Object Reference")))

(event `self.ReceiveTick`
  (params (DeltaSeconds :type "Float (single-precision)")))

(event `self.Box.OnComponentBeginOverlap`
  (params (OverlappedComponent :type "PrimitiveComponent Object Reference") (OtherActor :type "Actor Object Reference") (OtherComp :type "PrimitiveComponent Object Reference") (OtherBodyIndex :type Integer) (bFromSweep :type Boolean) (SweepResult :type "HitResult Structure (by ref)")))

(event `self.Cube.OnComponentBeginOverlap`
  (params (OverlappedComponent :type "PrimitiveComponent Object Reference") (OtherActor :type "Actor Object Reference") (OtherComp :type "PrimitiveComponent Object Reference") (OtherBodyIndex :type Integer) (bFromSweep :type Boolean) (SweepResult :type "HitResult Structure (by ref)")))

(fn `Debug_Heat`
  (if (`self.Debug`)
    (`TextRenderComponent.K2_SetText` (`self.Text_Comp`) (`KismetTextLibrary.Conv_DoubleToText` (`Heat_Component.Accumulated_Heat` (`self.Heat_Component`)) "HalfToEven"))
    (`TextRenderComponent.K2_SetText` (`self.Text_Comp_2`) (`KismetTextLibrary.Conv_DoubleToText` (`Heat_Component.Heat_Status_Param` (`self.Heat_Component`)) "HalfToEven"))))

(fn `UserConstructionScript`
  (if (`self.Debug`)
    (bind _returnvalue (`AddComponent|NODE_AddTextRenderComponent-5` :`RelativeTransform` (`KismetMathLibrary.MakeTransform` (60.0 35.0 -5.0))))
    (set `self.Text_Comp` _returnvalue)
    (bind _returnvalue_2 (`AddComponent|NODE_AddTextRenderComponent-6` :`RelativeTransform` (`KismetMathLibrary.MakeTransform` (60.0 35.0 25.0))))
    (set `self.Text_Comp_2` _returnvalue_2)
    (`self.Debug_Heat`)))
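; BP_Fire_Stream is a fire stream hazard that switches on only while all of its linked target buttons are active.
; At BeginPlay it binds to each valid target's activation-change delegate, then rechecks every target whenever one changes.
; Enabling turns on query collision on the flame trigger capsule and sets a damage-over-time timer.
; Disabling removes that collision and clears the timer.
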(event `self.ReceiveBeginPlay`
  (for _array_element (`self.Button_Targets`)
    (`/Engine/EditorBlueprintResources/StandardMacros.IsValid` _array_element
      (:`Is Valid`
        (add `/Game/Blueprints/BP_Button.Button_ActivationChange_Delegate` _array_element (`|CreateDelegate` :!event `Button_ActivationChange`))))))

(event `Button_ActivationChange`
  (params (new_value :type Boolean))
  (bind _result (`self.Is_All_Buttons_Active`))
  (if _result
    (`self.Enable_Fire`)
    (else
      (`self.Disable_Fire`))))

(event `Comp_OnAllCheckHeat`
  (params (heat_status :type "Float (double-precision)")))

(fn `Disable_Fire`
  (`PrimitiveComponent.SetCollisionEnabled` (`self.Flame_Trigger_Capsule`) "NoCollision")
  (`self.Clear_Dealing_DamageOverTime_Timer`))

(fn `Enable_Fire`
  (`PrimitiveComponent.SetCollisionEnabled` (`self.Flame_Trigger_Capsule`) "QueryOnly")
  (`self.Set_Dealing_DamageOverTime_Timer`))

(fn `Is_All_Buttons_Active`
  (returns (result :type Boolean))
  (for _array_element (`self.Button_Targets`)
    (if (not (`/Game/Blueprints/BP_Button.Is_Active` _array_element))
      (return false)))
  (return true))

(fn `UserConstructionScript`)
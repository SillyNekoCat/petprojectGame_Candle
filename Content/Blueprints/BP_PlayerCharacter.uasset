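; Player character Blueprint that uses GAS for melee attacks and blocking, grants starting abilities and deletes the SG_Tree save slot on BeginPlay.
; A line trace grabs "Grabable" objects with a PhysicsHandle; look input rotates them while view rotation stays locked, and distance can force release.
; Turn-in-place clamps aim-to-body yaw while idle and sets animation flags, gated by attack state.
; Overlapped pickups receive Interact; bound health handlers are empty.
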(event `self.ReceiveBeginPlay`
  (`self.Bind_Health_Events`)
  (set `CharacterMovementComponent.MaxWalkSpeed` (`.ReturnValue` (`AbilitySystemComponent.GetGameplayAttributeValue` (`self.AbilitySystem_Comp`) (struct :`AttributeName` "Move_Speed" :`Attribute` "/Script/Living_Candle.Movement_AttributeSet:Move_Speed" :`AttributeOwner` "/Script/CoreUObject.Class'/Script/Living_Candle.Movement_AttributeSet'"))) (`self.CharacterMovement`))
  (`self.Give_StartAbilities` (`self.Ability Class`) (`self.AbilitySystem_Comp`))
  (`GameplayStatics.DeleteGameInSlot` "SG_Tree"))

(event `self.ReceiveTick`
  (params (DeltaSeconds :type "Float (single-precision)"))
  (bind _physicshandle (`self.PhysicsHandle`))
  (if (`self.Is_GrabbingObj`)
    (`PhysicsHandleComponent.SetTargetRotation` _physicshandle (`.TargetRotation` (`PhysicsHandleComponent.GetTargetLocationAndRotation` _physicshandle)))
    (`Controller.SetControlRotation` (`self.GetLocalViewingPlayerController`) (`self.OnGrab_LockRotation`))
    (if (`self.Valid_DistanceBetween_GrabbedObjAndThisActor`)
      (`self.PhysHanlde_Release`))))

(event `self.CapsuleComponent.OnComponentBeginOverlap`
  (params (OverlappedComponent :type "PrimitiveComponent Object Reference") (OtherActor :type "Actor Object Reference") (OtherComp :type "PrimitiveComponent Object Reference") (OtherBodyIndex :type Integer) (bFromSweep :type Boolean) (SweepResult :type "HitResult Structure (by ref)"))
  ;[1 1 1] Interaction
  (bind _aspickup_able_item (cast `PickupAble_Item` OtherActor))
  (`Interactable_Actor.Interact` _aspickup_able_item self))

(event `EnhancedInput|/Game/Input/Actions/IA_Use`
  (params (ActionValue :type Boolean) (ElapsedSeconds :type "Float (double-precision)") (TriggeredSeconds :type "Float (double-precision)") (InputAction :type "InputAction Object Reference" :default "/Game/Input/Actions/IA_Use.IA_Use"))
  ;[1 1 1] Interaction
  (:`Triggered`
    (if (`self.Is_GrabbingObj`)
      (`self.PhysHanlde_Release`)
      (else
        (`self.PhysHanlde_Grab`)))))

(event `EnhancedInput|/Game/Input/Actions/IA_Look`
  (params (ActionValue :type "Vector2D Structure") (ElapsedSeconds :type "Float (double-precision)") (TriggeredSeconds :type "Float (double-precision)") (InputAction :type "InputAction Object Reference" :default "/Game/Input/Actions/IA_Look.IA_Look"))
  ;[1 1 1] Interaction
  (:`Triggered`
    (`self.PhysHandle_Rotate` (* ActionValue (2.0 2.0)))))

(event `EnhancedInput|/Game/Input/Actions/IA_Heat_Item`
  (params (ActionValue :type Boolean) (ElapsedSeconds :type "Float (double-precision)") (TriggeredSeconds :type "Float (double-precision)") (InputAction :type "InputAction Object Reference" :default "/Game/Input/Actions/IA_Heat_Item.IA_Heat_Item"))
  ;[1 1 1] Interaction
  (:`Triggered`
    (set `self.Is_Heating_Item` ActionValue)))

(event `EnhancedInput|/Game/Input/Actions/IA_Attack`
  (params (ActionValue :type Boolean) (ElapsedSeconds :type "Float (double-precision)") (TriggeredSeconds :type "Float (double-precision)") (InputAction :type "InputAction Object Reference" :default "/Game/Input/Actions/IA_Attack.IA_Attack"))
  ;[1 1 1] Abilities
  (:`Triggered`
    (`AbilitySystemComponent.TryActivateAbilitiesByTag` (`self.AbilitySystem_Comp`) (`BlueprintGameplayTagLibrary.MakeLiteralGameplayTagContainer` (struct :`GameplayTags` (struct :`(TagName` "Ability.Melee_Attack.Primary")))) true)))

(event `EnhancedInput|/Game/Input/Actions/IA_AltAttack`
  (params (ActionValue :type Boolean) (ElapsedSeconds :type "Float (double-precision)") (TriggeredSeconds :type "Float (double-precision)") (InputAction :type "InputAction Object Reference" :default "/Game/Input/Actions/IA_AltAttack.IA_AltAttack"))
  ;[1 1 1] Abilities
  (:`Triggered`
    (if (not (`NavMovementComponent.IsFalling` (`self.CharacterMovement`)))
      (`AbilitySystemComponent.TryActivateAbilitiesByTag` (`self.AbilitySystem_Comp`) (`BlueprintGameplayTagLibrary.MakeLiteralGameplayTagContainer` (struct :`GameplayTags` (struct :`(TagName` "Ability.Melee_Attack.Second")))) true))))

(event `EnhancedInput|/Game/Input/Actions/IA_Blocking`
  (params (ActionValue :type Boolean) (ElapsedSeconds :type "Float (double-precision)") (TriggeredSeconds :type "Float (double-precision)") (InputAction :type "InputAction Object Reference" :default "/Game/Input/Actions/IA_Blocking.IA_Blocking"))
  ;[1 1 1] Abilities
  (:`Triggered`
    (if ActionValue
      (`AbilitySystemComponent.TryActivateAbilitiesByTag` (`self.AbilitySystem_Comp`) (`BlueprintGameplayTagLibrary.MakeLiteralGameplayTagContainer` (struct :`GameplayTags` (struct :`(TagName` "Ability.Blocking.Activate_Block")))) true)
      (else
        (`AbilitySystemComponent.TryActivateAbilitiesByTag` (`self.AbilitySystem_Comp`) (`BlueprintGameplayTagLibrary.MakeLiteralGameplayTagContainer` (struct :`GameplayTags` (struct :`(TagName` "Ability.Blocking.Cancel_Block")))) true)))))

(event `Bind_Health_Events`
  (bind _returnvalue (`AbilitySystemComponent.GetAttributeSet` (`self.AbilitySystem_Comp`) "/Script/Living_Candle.Base_AttributeSet"))
  (bind _asbase_attribute_set (cast `Base_AttributeSet` _returnvalue))
  (add `Base_AttributeSet.On_RecieveDamage` _asbase_attribute_set (`|CreateDelegate` :!event `On_RecieveDamage_Event`))
  (add `Base_AttributeSet.On_Health_Changed` _asbase_attribute_set (`|CreateDelegate` :!event `On_Health_Changed_Event`)))

(event `On_RecieveDamage_Event`
  (params (EffectInstigator :type "Actor Object Reference") (EffectCauser :type "Actor Object Reference") (Damage_Info :type "Damage_Info Structure")))

(event `On_Health_Changed_Event`
  (params (EffectInstigator :type "Actor Object Reference") (EffectCauser :type "Actor Object Reference") (DamageTag :type "GameplayTag Structure") (Magnitude :type "Float (single-precision)") (OldValue :type "Float (single-precision)") (NewValue :type "Float (single-precision)")))

(event `EnhancedInput|/Game/Input/Actions/IA_Move`
  (params (ActionValue :type "Vector2D Structure") (ElapsedSeconds :type "Float (double-precision)") (TriggeredSeconds :type "Float (double-precision)") (InputAction :type "InputAction Object Reference" :default "/Game/Input/Actions/IA_Move.IA_Move")))

(event `EnhancedInput|/Game/Input/Actions/IA_Move`
  (params (ActionValue :type "Vector2D Structure") (ElapsedSeconds :type "Float (double-precision)") (TriggeredSeconds :type "Float (double-precision)") (InputAction :type "InputAction Object Reference" :default "/Game/Input/Actions/IA_Move.IA_Move"))
  (bind _is_grabbingobj (`self.Is_GrabbingObj`))
  (bind _charactermovement (`self.CharacterMovement`))
  ;[1 1 1] Turn in place
  (:`Triggered`
    (if _is_grabbingobj
      (set `CharacterMovementComponent.bUseControllerDesiredRotation` false _charactermovement :!label _label)
      (set `self.Move_Input` false)
      (elif (`Attack_Comp.Is_Attacking` (`self.Attack_Compo`))
        (if (`Attack_Comp.Can_AttackAndMove` (`self.Attack_Compo`))
          (set `self.Move_Input` true :!label _label_2)
          (set `CharacterMovementComponent.bUseControllerDesiredRotation` true _charactermovement)
          (set `self.Is_Turn_Left` false)
          (set `self.Is_Turn_Right` false))
        (else
          (goto _label_2)))))
  (:`Completed`
    (if _is_grabbingobj
      (goto _label)
      (else
        (goto _label)))))

(event `EnhancedInput|/Game/Input/Actions/IA_Look`
  (params (ActionValue :type "Vector2D Structure") (ElapsedSeconds :type "Float (double-precision)") (TriggeredSeconds :type "Float (double-precision)") (InputAction :type "InputAction Object Reference" :default "/Game/Input/Actions/IA_Look.IA_Look"))
  ;[1 1 1] Turn in place
  (:`Triggered`
    (if (not (`self.Is_GrabbingObj`))
      (bind _is_turn_end (`self.Calc_Turn`))
      (if _is_turn_end
        ;;[1 1 1] How long turn animation will playing after end of turning
        (`KismetSystemLibrary.Delay` 0.09)
        (set `self.Is_Turn_Left` false)
        (set `self.Is_Turn_Right` false)))))

(event `EnhancedInput|/Game/Input/Actions/IA_Look_X`
  (params (ActionValue :type "Float (double-precision)") (ElapsedSeconds :type "Float (double-precision)") (TriggeredSeconds :type "Float (double-precision)") (InputAction :type "InputAction Object Reference" :default "/Game/Input/Actions/IA_Look_X.IA_Look_X")))

(event `EnhancedInput|/Game/Input/Actions/IA_Look_Y`
  (params (ActionValue :type "Float (double-precision)") (ElapsedSeconds :type "Float (double-precision)") (TriggeredSeconds :type "Float (double-precision)") (InputAction :type "InputAction Object Reference" :default "/Game/Input/Actions/IA_Look_Y.IA_Look_Y")))

(fn `Calc_Turn`
  (returns (is_turn_end :type Boolean))
  (bind _returnvalue (`self.GetBaseAimRotation`))
  (bind (_returnvalue_roll _returnvalue_pitch _returnvalue_yaw) (`KismetMathLibrary.BreakRotator` (`KismetMathLibrary.NormalizedDeltaRotator` (`self.GetBaseAimRotation`) (`self.K2_GetActorRotation`))))
  (if (`self.Move_Input`)
    _
    (elif (`Attack_Comp.Is_Attacking` (`self.Attack_Compo`))
      (if (`Attack_Comp.Can_AttackAndMove` (`self.Attack_Compo`))
        (`|ExecutionSequence` :!label _label
          (:`then_0`
            (if (> _returnvalue_yaw 80.0)
              (set `self.Is_Turn_Right` true)
              (`self.K2_SetActorRotation` (`KismetMathLibrary.MakeRotator` 0.0 0.0 (- (.yaw _returnvalue) 79.0)))))
          (:`then_1`
            (if (< _returnvalue_yaw -80.0)
              (set `self.Is_Turn_Left` true)
              (`self.K2_SetActorRotation` (`KismetMathLibrary.MakeRotator` 0.0 0.0 (+ (.yaw _returnvalue) 79.0)))))
          (:`then_2`
            (return (`KismetMathLibrary.NearlyEqual_FloatFloat` _returnvalue_yaw 0.0 80.0)))))
      (else
        (goto _label)))))

(fn `Give_StartAbilities`
  (params (ability_classes :type "Array of GameplayAbility Class Reference") (target_asc :type "AbilitySystemComponent Object Reference"))
  (for _array_element ability_classes
    (`AbilitySystemComponent.K2_GiveAbility` target_asc _array_element 0 -1)))

(fn `PhysHandle_Rotate`
  (params (InVec :type "Vector2D Structure"))
  (bind (_x _y) (`KismetMathLibrary.BreakVector2D` InVec))
  (bind (_targetlocation _targetrotation) (`PhysicsHandleComponent.GetTargetLocationAndRotation` (`self.PhysicsHandle`)))
  (if (`self.Is_GrabbingObj`)
    (`PhysicsHandleComponent.SetTargetRotation` (`self.PhysicsHandle`) (`KismetMathLibrary.MakeRotator` (+ _x (.roll _targetrotation)) (+ _y (.pitch _targetrotation)) (.yaw _targetrotation)))))

(fn `PhysHanlde_Grab`
  (bind (_start _end) (`self.GrabTrace_Locations`))
  (bind (_outhit _returnvalue) (`KismetSystemLibrary.LineTraceSingle` :`Start` _start :`End` _end :`TraceChannel` "TraceTypeQuery1" :`DrawDebugType` "ForDuration"))
  (if _returnvalue
    (bind (_bblockinghit _binitialoverlap _time _distance _location _impactpoint _normal _impactnormal _physmat _hitactor _hitcomponent) (`GameplayStatics.BreakHitResult` _outhit))
    (if (`self.ActorHasTag` _hitactor "Grabable")
      (`PhysicsHandleComponent.GrabComponentAtLocationWithRotation` :`self` (`self.PhysicsHandle`) :`Component` _hitcomponent :`Location` (`self.K2_GetActorLocation` _hitactor))
      (`/Engine/EditorBlueprintResources/StandardMacros.IsValid` (`PhysicsHandleComponent.GetGrabbedComponent` (`self.PhysicsHandle`))
        (:`Is Valid`
          (set `self.Is_GrabbingObj` true)
          (set `self.OnGrab_LockRotation` (`self.GetBaseAimRotation`)))))))

(fn `PhysHanlde_Release`
  (`PhysicsHandleComponent.ReleaseComponent` (`self.PhysicsHandle`))
  (set `self.Is_GrabbingObj` false))

(fn `Set_CanAttackAndMove`
  (params (`new value` :type Boolean))
  (set `Attack_Comp.Can_AttackAndMove` `new value` (`self.Attack_Compo`))
  (`self.OnCanAttackAndMoveChange` `new value`))

(fn `Set_Good_Player_Scale`)

(fn `UserConstructionScript`)
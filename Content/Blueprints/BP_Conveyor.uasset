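; Conveyor belt actor that carries tagged actors along its mesh's forward vector and scrolls a dynamic belt material to match its speed.
; Tick runs only while tagged actors overlap the interact box, offsetting movable actors each frame, with sweep for non-physics ones.
; Overlapping conveyors use each other's ignore lists to claim shared actors.
; Actors leaving the last belt receive an impulse, applied through physics or character movement.
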(event `self.ReceiveTick`
  (params (DeltaSeconds :type "Float (single-precision)"))
  (bind _overlappingactors (`PrimitiveComponent.GetOverlappingActors` (`self.Interact_Box`) null))
  (bind _is_contains_tag (`self.AtLeastOneActor_ContainsTag` _overlappingactors (`self.Move_Tag`)))
  (if _is_contains_tag
    (`self.ArrayFilter` _overlappingactors)
    (for _array_element (`self.Tick_Overlapping_Actors`)
      (`self.MoveObject` _array_element))
    (`KismetArrayLibrary.Array_Clear` (`self.Tick_Overlapping_Actors`))
    (`KismetArrayLibrary.Array_Clear` (`self.Ignore_Actors`))
    (else
      (`self.SetActorTickEnabled` false)
      (`KismetArrayLibrary.Array_Clear` (`self.Tick_Overlapping_Actors`))
      (`KismetArrayLibrary.Array_Clear` (`self.Ignore_Actors`)))))

(event `self.Interact_Box.OnComponentBeginOverlap`
  (params (OverlappedComponent :type "PrimitiveComponent Object Reference") (OtherActor :type "Actor Object Reference") (OtherComp :type "PrimitiveComponent Object Reference") (OtherBodyIndex :type Integer) (bFromSweep :type Boolean) (SweepResult :type "HitResult Structure (by ref)"))
  (if (`KismetArrayLibrary.Array_Contains` (`Actor.Tags` OtherActor) (`self.Move_Tag`))
    (`self.SetActorTickEnabled` true)))

(event `self.Interact_Box.OnComponentEndOverlap`
  (params (OverlappedComponent :type "PrimitiveComponent Object Reference") (OtherActor :type "Actor Object Reference") (OtherComp :type "PrimitiveComponent Object Reference") (OtherBodyIndex :type Integer))
  (if (`self.Is_Actor_Movable` OtherActor)
    (for _array_element (`self.GetOverlappingActors` OtherActor "BP_Conveyor_C")
      (bind _asbp_conveyor (cast `/Game/Blueprints/BP_Conveyor` _array_element)
        (:`then`
          (if (!= _asbp_conveyor self)
            (`KismetArrayLibrary.Array_RemoveItem` (`/Game/Blueprints/BP_Conveyor.Ignore_Actors` _asbp_conveyor) OtherActor)))
        (:`CastFailed`
          (`KismetSystemLibrary.PrintString` "Hello"))))
    (if (== (`KismetArrayLibrary.Array_Length` (`self.GetOverlappingActors` OtherActor "BP_Conveyor_C")) 0)
      (bind _asprimitive_component (cast `PrimitiveComponent` (`Actor.RootComponent` OtherActor)))
      (if (`SceneComponent.IsAnySimulatingPhysics` _asprimitive_component)
        (`PrimitiveComponent.AddImpulse` _asprimitive_component (* (`SceneComponent.GetForwardVector` (`self.MeshConveyor0`)) (/ (`self.Speed_X`) 1.5)) "None" true)
        (else
          (`CharacterMovementComponent.AddImpulse` (`self.GetComponentByClass` OtherActor "/Script/Engine.CharacterMovementComponent") (* (`SceneComponent.GetForwardVector` (`self.MeshConveyor0`)) (/ (* (`self.Speed_X`) (`self.Character_Impulse_Multiplyer`)) 1.5)) true))))))

(fn `ArrayFilter`
  (params (InputPin :type "Array of Actor Object Reference"))
  (for _array_element InputPin
    (if (`self.Is_Actor_Movable` _array_element)
      (`KismetArrayLibrary.Array_AddUnique` (`self.Tick_Overlapping_Actors`) _array_element)
      (for _array_element_2 (`self.GetOverlappingActors` _array_element "BP_Conveyor_C")
        (bind _asbp_conveyor (cast `/Game/Blueprints/BP_Conveyor` _array_element_2))
        (if (!= _asbp_conveyor self)
          (`KismetArrayLibrary.Array_AddUnique` (`/Game/Blueprints/BP_Conveyor.Ignore_Actors` _asbp_conveyor) _array_element))))))

(fn `AtLeastOneActor_ContainsTag`
  (params (Array :type "Array of Actor Object Reference") (InputPin :type Name))
  (returns (is_contains_tag :type Boolean))
  (for _array_element Array
    (bind _returnvalue (`KismetArrayLibrary.Array_Contains` (`Actor.Tags` _array_element) InputPin))
    (if _returnvalue
      (return _returnvalue))))

(fn `MaterialSetup_TopBottom`
  (params (Comp :type "PrimitiveComponent Object Reference") (MatElemIndex :type Integer))
  (bind _matinst_topbottom (`self.MatInst_TopBottom`))
  (bind _returnvalue (`PrimitiveComponent.CreateDynamicMaterialInstance` Comp MatElemIndex "/Game/Materials/M_Conveyor.M_Conveyor" "None"))
  (set `self.MatInst_TopBottom` _returnvalue)
  (`PrimitiveComponent.SetMaterial` Comp MatElemIndex _matinst_topbottom)
  (`MaterialInstanceDynamic.SetVectorParameterValue` _matinst_topbottom "Color" (`self.Color`))
  (`MaterialInstanceDynamic.SetScalarParameterValue` _matinst_topbottom "Scale_X" (.x (`self.GetActorScale3D`)))
  (`self.SetMatParam_SpeedX` (`self.Speed_X`) _matinst_topbottom))

(fn `MoveObject`
  (params (elem :type "Actor Object Reference"))
  (bind _returnvalue (* (`SceneComponent.GetForwardVector` (`self.MeshConveyor0`)) (* (`GameplayStatics.GetWorldDeltaSeconds`) (`self.Speed_X`))))
  (if (`self.Is_Actor_Movable` elem)
    (if (`SceneComponent.IsAnySimulatingPhysics` (`Actor.RootComponent` elem))
      (`self.K2_AddActorWorldOffset` elem _returnvalue false false)
      (else
        ;[1 1 1] Move Characters
        (`self.K2_AddActorWorldOffset` elem _returnvalue true false)))))

(fn `SetMatParam_SpeedX`
  (params (new_speed :type "Float (single-precision)") (material_instance_dynamic :type "MaterialInstanceDynamic Object Reference"))
  (set `self.Speed_X` new_speed)
  (`MaterialInstanceDynamic.SetScalarParameterValue` material_instance_dynamic "Speed_X" (* (/ (`self.Speed_X`) (`self.MaterialSpeed_Divider`)) -1.0)))

(fn `UserConstructionScript`
  (`self.MaterialSetup_TopBottom` (`self.MeshConveyor0`)))
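; GA_Dash is a Gameplay Ability that picks a dash direction and hands off to its parent ability.
; Activation proceeds only when the avatar is neither falling nor attacking, as read from its movement component and Attack_Comp.
; Direction comes from the last movement input, or from the flattened base aim forward vector when there is none.
; The parent's ActivateAbility then runs, so the dash movement itself lives outside this graph.
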(event `self.K2_ActivateAbility`
  (bind _returnvalue (`self.GetAvatarActorFromActorInfo`))
  (bind _instigator (`Actor.Instigator` _returnvalue))
  (bind _returnvalue_2 (`Pawn.GetLastMovementInputVector` _instigator))
  (if (and (not (`NavMovementComponent.IsFalling` (`Actor.GetComponentByClass` _returnvalue "/Script/Engine.CharacterMovementComponent"))) (not (`Attack_Comp.Is_Attacking` (`Actor.GetComponentByClass` _returnvalue "/Script/Living_Candle.Attack_Comp"))))
    (if (== _returnvalue_2 (0.0 0.0 0.0))
      (set `self.Direction` (`KismetMathLibrary.Vector_Normal2D` (`KismetMathLibrary.GetForwardVector` (`Pawn.GetBaseAimRotation` _instigator))))
      (else
        (set `self.Direction` _returnvalue_2)))
    (`parent.K2_ActivateAbility`)))
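; Static Gameplay Cue that toggles whether the player character can attack and move.
; OnActive casts the target to BP_PlayerCharacter and calls SetCanAttackAndMove with true, and OnRemove does the same with false.
; Both call the parent handler only when the cast succeeds.
; Older nodes that set CanAttack directly on Attack_Comp remain in both graphs but never run.
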(fn `OnActive`
  (params (MyTarget :type "Actor Object Reference") (Parameters :type "GameplayCueParameters Structure (by ref)"))
  (returns (ReturnValue :type Boolean))
  (bind _asbp_player_character (cast `/Game/Blueprints/BP_PlayerCharacter` MyTarget))
  (`/Game/Blueprints/BP_PlayerCharacter.Set_CanAttackAndMove` _asbp_player_character true)
  (return (`parent.OnActive` MyTarget Parameters)))

(fn `OnRemove`
  (params (MyTarget :type "Actor Object Reference") (Parameters :type "GameplayCueParameters Structure (by ref)"))
  (returns (ReturnValue :type Boolean))
  (bind _asbp_player_character (cast `/Game/Blueprints/BP_PlayerCharacter` MyTarget))
  (`/Game/Blueprints/BP_PlayerCharacter.Set_CanAttackAndMove` _asbp_player_character false)
  (return (`parent.OnRemove` MyTarget Parameters)))
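; BP_LogicDoor is a door that opens and closes according to the heat status broadcast by a linked Target.
; On BeginPlay it stores the Cube's starting relative location and binds to the Target's OnCheckHeat delegate.
; A heat status at or above the threshold plays a Timeline that lerps the Cube upward; anything lower reverses the Timeline to close it.
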(event `self.ReceiveBeginPlay`
  (set `self.Cube Start Relative Location` (`SceneComponent.RelativeLocation` (`self.Cube`)))
  (add `Heat_Actor.OnCheckHeat_Delegate` (`self.Target`) (delegate `OnCheckHeat_Delegate_Event`)))

(event `OnCheckHeat_Delegate_Event`
  (params (heat_status :type "Float (double-precision)"))
  (if (>= heat_status 1.0)
    (bind (_direction _door_relative_location) (`Timeline|Timeline` :!label _label)
      (:`Update`
        (`SceneComponent.K2_SetRelativeLocation` (`self.Cube`) (`KismetMathLibrary.VLerp` (`self.Cube Start Relative Location`) (+ (`self.Cube Start Relative Location`) (0.0 0.0 200.0)) _door_relative_location) false false)))
    (else
      (goto _label :!via `Reverse`))))

(fn `UserConstructionScript`)
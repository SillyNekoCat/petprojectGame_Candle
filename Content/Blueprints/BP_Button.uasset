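; Pressure button actor that switches between active and inactive in Hold or Toggle mode and broadcasts activation changes through a delegate.
; The first actor entering the interact box plays a timeline that presses the mesh, and the last one leaving reverses it.
; The timeline drives optional glow and color lerps on a dynamic material; Hold follows the press, while Toggle flips on each completed press.
; IsActiveFromStart sets the initial state and inverts the activation logic.
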(event `self.ReceiveBeginPlay`
  (bind _is_active_fromstart (`self.Is_Active_FromStart`))
  (switch `/Game/Blueprints/Enums/Enum_ButtonInteractionType` (`self.Button_Interaction_Type`)
    (:`NewEnumerator2`
      _)
    (:`NewEnumerator6`
      (if _is_active_fromstart
        (`self.Swap_Colors`))))
  (set `self.Is_Active` _is_active_fromstart)
  (`self.Button_ActivationChange_Delegate` _is_active_fromstart))

(event `self.Interact_Box.OnComponentBeginOverlap`
  (params (OverlappedComponent :type "PrimitiveComponent Object Reference") (OtherActor :type "Actor Object Reference") (OtherComp :type "PrimitiveComponent Object Reference") (OtherBodyIndex :type Integer) (bFromSweep :type Boolean) (SweepResult :type "HitResult Structure (by ref)"))
  (bind _overlappingactors (`PrimitiveComponent.GetOverlappingActors` (`self.Interact_Box`) null))
  (if (and (not (`KismetArrayLibrary.Array_Contains` (`self.Already_Overlap`) OtherActor)) (== (`KismetArrayLibrary.Array_Length` _overlappingactors) 1))
    (set `self.Already_Overlap` _overlappingactors)
    (bind (_direction _button_relative_location) (`Timeline|Timeline` :!label _label)
      (:`Update`
        (`|ExecutionSequence`
          (:`then_0`
            (if (`self.Glow_OnPush`)
              (`MaterialInstanceDynamic.SetScalarParameterValue` (`self.MatButton`) "Glow" _button_relative_location)))
          (:`then_1`
            (`SceneComponent.K2_SetRelativeLocation` (`self.Button`) (`KismetMathLibrary.VLerp` (`self.Cube Start Relative Location`) (+ (`self.Cube Start Relative Location`) (`self.End_Offset`)) _button_relative_location) false false)
            (switch `/Game/Blueprints/Enums/Enum_ButtonInteractionType` (`self.Button_Interaction_Type`)
              (:`NewEnumerator2`
                (`self.SetColor_Hold` _button_relative_location))
              (:`NewEnumerator6`
                (switch `ETimelineDirection` _direction
                  (:`Forward`
                    (`self.SetColor_Toggle` _button_relative_location))
                  (:`Backward`
                    (`/Engine/EditorBlueprintResources/StandardMacros.Gate` false :!label _label_2
                      (:`Exit`
                        (`self.SetColor_Toggle` _button_relative_location true))))))))))
      (:`Finished`
        (switch `/Game/Blueprints/Enums/Enum_ButtonInteractionType` (`self.Button_Interaction_Type`)
          (:`NewEnumerator2`
            (switch `ETimelineDirection` _direction
              (:`Forward`
                (`self.Call_Change_Activation` true))
              (:`Backward`
                (`self.Call_Change_Activation` false))))
          (:`NewEnumerator6`
            (switch `ETimelineDirection` _direction
              (:`Forward`
                (`|ExecutionSequence`
                  (:`then_0`
                    (goto _label_2 :!via `Close`))
                  (:`then_1`
                    (bind _isa (`/Engine/EditorBlueprintResources/StandardMacros.FlipFlop`)
                      (:`A`
                        _)
                      (:`B`
                        _))
                    (`self.Call_Change_Activation` _isa))))
              (:`Backward`
                (goto _label_2 :!via `Open`)))))))))

(event `self.Interact_Box.OnComponentEndOverlap`
  (params (OverlappedComponent :type "PrimitiveComponent Object Reference") (OtherActor :type "Actor Object Reference") (OtherComp :type "PrimitiveComponent Object Reference") (OtherBodyIndex :type Integer))
  (bind _overlappingactors (`PrimitiveComponent.GetOverlappingActors` (`self.Interact_Box`) null))
  (set `self.Already_Overlap` _overlappingactors)
  (if (`KismetArrayLibrary.Array_IsEmpty` _overlappingactors)
    (goto _label :!via `Reverse`)))

(fn `Call_Change_Activation`
  (params (is_active :type Boolean))
  (if (`self.Is_Active_FromStart`)
    (bind _output_get (set `self.Is_Active` (not is_active)))
    (`self.Button_ActivationChange_Delegate` _output_get)
    (else
      (bind _output_get_2 (set `self.Is_Active` is_active))
      (`self.Button_ActivationChange_Delegate` _output_get_2))))

(fn `SetColor_Hold`
  (params (Alpha :type "Float (single-precision)"))
  (if (`self.Is_Active_FromStart`)
    (`MaterialInstanceDynamic.SetVectorParameterValue` (`self.MatButton`) "Color" (`KismetMathLibrary.LinearColorLerp` (`self.Active_Color`) (`self.NonActive_Color`) Alpha))
    (else
      (`MaterialInstanceDynamic.SetVectorParameterValue` (`self.MatButton`) "Color" (`KismetMathLibrary.LinearColorLerp` (`self.NonActive_Color`) (`self.Active_Color`) Alpha)))))

(fn `SetColor_Toggle`
  (params (Alpha :type "Float (single-precision)") (reverse :type Boolean))
  (if (`self.Is_Active_FromStart`)
    (if (not (`self.Is_Active`))
      (`MaterialInstanceDynamic.SetVectorParameterValue` (`self.MatButton`) "Color" (`KismetMathLibrary.LinearColorLerp` (`self.Active_Color`) (`self.NonActive_Color`) Alpha) :!label _label)
      (else
        (`MaterialInstanceDynamic.SetVectorParameterValue` (`self.MatButton`) "Color" (`KismetMathLibrary.LinearColorLerp` (`self.NonActive_Color`) (`self.Active_Color`) Alpha) :!label _label_2)))
    (elif (`self.Is_Active`)
      (goto _label)
      (else
        (goto _label_2)))))

(fn `Swap_Colors`
  (locals (previous_active_color :type "LinearColor Structure"))
  (set `local.previous_active_color` (`self.Active_Color`))
  (set `self.Active_Color` (`self.NonActive_Color`))
  (set `self.NonActive_Color` (`local.previous_active_color`)))

(fn `UserConstructionScript`
  (set `self.Cube Start Relative Location` (`SceneComponent.RelativeLocation` (`self.Button`)))
  (bind _returnvalue (`KismetMaterialLibrary.CreateDynamicMaterialInstance` "/Game/Materials/M_Overlay_ButtonActivation.M_Overlay_ButtonActivation"))
  (bind _output_get (set `self.MatButton` _returnvalue))
  (`PrimitiveComponent.SetMaterial` (`self.Button`) 0 _output_get)
  (`MaterialInstanceDynamic.SetScalarParameterValue` (`self.MatButton`) "Opacity" (`self.Start_Opacity`))
  (`MaterialInstanceDynamic.SetScalarParameterValue` (`self.MatButton`) "Glow" (`KismetMathLibrary.Conv_BoolToDouble` (`self.Always_Glow`)))
  (if (`self.Is_Active_FromStart`)
    (`MaterialInstanceDynamic.SetVectorParameterValue` (`self.MatButton`) "Color" (`self.Active_Color`))
    (else
      (`MaterialInstanceDynamic.SetVectorParameterValue` (`self.MatButton`) "Color" (`self.NonActive_Color`)))))
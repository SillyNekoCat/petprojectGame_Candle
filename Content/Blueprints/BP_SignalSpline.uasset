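; BP_SignalSpline is a spline actor that tiles a mesh along its path and binds to a target button and heat actor.
; The Construction Script adds spline mesh segments by section length, optionally derived from X scale, with an option to drop the last partial segment.
; Segment tangents are clamped to section length.
; BeginPlay binds the button activation and heat check delegates, but both handlers are empty here.
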(event `self.ReceiveBeginPlay`
  (bind _button_target (`self.Button_Target`))
  (bind _heatactor_target (`self.HeatActor_Target`))
  (`|ExecutionSequence`
    (:`then_0`
      (`/Engine/EditorBlueprintResources/StandardMacros.IsValid` _button_target
        (:`Is Valid`
          (add `/Game/Blueprints/BP_Button.Button_ActivationChange_Delegate` _button_target (`|CreateDelegate` :!event `Button_ActivationChange`))
          (set `self.Target Button Interaction Type` (`/Game/Blueprints/BP_Button.Button_Interaction_Type` _button_target)))))
    (:`then_1`
      (`/Engine/EditorBlueprintResources/StandardMacros.IsValid` _heatactor_target
        (:`Is Valid`
          (add `Heat_Actor.OnCheckHeat_Delegate` _heatactor_target (`|CreateDelegate` :!event `Event_CheckHeat`)))))))

(event `Button_ActivationChange`
  (params (new_value :type Boolean)))

(event `Event_CheckHeat`
  (params (heat_status :type "Float (double-precision)")))

(fn `UserConstructionScript`
  (locals (loop_index :type Integer))
  (bind _returnvalue_x (`KismetMathLibrary.BreakVector` (`self.GetActorScale3D`)))
  (bind _returnvalue (`self.Amount of Spline Meshes`))
  (bind _loop_index (`local.loop_index`))
  (bind (_position _tangent) (`self.Get Start Pos and Tangent` _loop_index))
  (bind (_position_2 _tangent_2) (`self.Get End Pos and Tangent` _loop_index))
  (if (`self.IsAllowScaling`)
    (set `self.Section_Length` (* _returnvalue_x 100.0)))
  (if (`self.IsFullLengthMeshes`)
    (for _index (range _returnvalue)
      (set `local.loop_index` _index)
      (bind _returnvalue_2 (`AddComponent|NODE_AddSplineMeshComponent-0` :!label _label))
      (`StaticMeshComponent.SetStaticMesh` _returnvalue_2 (`self.SplineMesh`))
      (`SplineMeshComponent.SetForwardAxis` _returnvalue_2 "X" true)
      (`SplineMeshComponent.SetStartAndEnd` _returnvalue_2 _position _tangent _position_2 _tangent_2 true)
      (`PrimitiveComponent.SetCollisionEnabled` _returnvalue_2 (`self.CollisionType`)))
    (else
      (for _index_2 (range (+ _returnvalue 1))
        (set `local.loop_index` _index_2)
        (goto _label)))))
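; Test AI character that uses a Gameplay Ability System attribute set to react to health changes and death.
; On BeginPlay it caches the Base_AttributeSet from its ability system component and binds its damage, health-changed and health-zero delegates.
; Health changes print the damage tag and magnitude, zero health destroys the actor, and the damage-taken handler is empty.
; A helper function sets the movement component's max walk speed.
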(event `self.ReceiveTick`
  (params (DeltaSeconds :type "Float (single-precision)")))

(event `self.ReceiveBeginPlay`
  (bind _asc_baseattributeset (`self.asc_BaseAttributeSet`))
  (`|ExecutionSequence`
    (:`then_0`
      (bind _returnvalue (`AbilitySystemComponent.GetAttributeSet` (`self.AbilitySystem_Comp`) "/Script/Living_Candle.Base_AttributeSet"))
      (bind _asbase_attribute_set (cast `Base_AttributeSet` _returnvalue))
      (set `self.asc_BaseAttributeSet` _asbase_attribute_set))
    (:`then_1`
      (add `Base_AttributeSet.On_Damage_Take` _asc_baseattributeset (delegate `On_Damage_Take_Event_1`))
      (add `Base_AttributeSet.On_Health_Changed` _asc_baseattributeset (delegate `On_Health_Changed_Event`))
      (add `Base_AttributeSet.On_Health_Zero` _asc_baseattributeset (delegate `On_Health_Zero_Event`)))))

(event `On_Damage_Take_Event_1`
  (params (EffectInstigator :type "Actor Object Reference") (EffectCauser :type "Actor Object Reference") (DamageTag :type "GameplayTag Structure") (Magnitude :type "Float (single-precision)") (OldValue :type "Float (single-precision)") (NewValue :type "Float (single-precision)")))

(event `On_Health_Changed_Event`
  (params (EffectInstigator :type "Actor Object Reference") (EffectCauser :type "Actor Object Reference") (DamageTag :type "GameplayTag Structure") (Magnitude :type "Float (single-precision)") (OldValue :type "Float (single-precision)") (NewValue :type "Float (single-precision)"))
  (`KismetSystemLibrary.PrintString` (`KismetStringLibrary.Concat_StrStr` (`KismetStringLibrary.Conv_NameToString` (`BlueprintGameplayTagLibrary.GetTagName` DamageTag)) "  " " : " (`KismetStringLibrary.Conv_DoubleToString` Magnitude))))

(event `On_Health_Zero_Event`
  (params (EffectInstigator :type "Actor Object Reference") (EffectCauser :type "Actor Object Reference") (DamageTag :type "GameplayTag Structure") (Magnitude :type "Float (single-precision)") (OldValue :type "Float (single-precision)") (NewValue :type "Float (single-precision)"))
  (`self.K2_DestroyActor`))

(fn `Update Walk Speed`
  (params (NewWalkSpeed :type "Float (double-precision)"))
  (set `CharacterMovementComponent.MaxWalkSpeed` NewWalkSpeed (`self.CharacterMovement`)))

(fn `UserConstructionScript`)